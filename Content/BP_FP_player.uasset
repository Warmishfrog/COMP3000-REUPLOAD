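; BP_FP_player is the first-person player Blueprint that manages game-flow menus and the match timer.
; Death, level-up, Escape and victory each pause the game, add their widget and switch to UI-only input with a cursor, while BeginPlay shows a jump message.
; A Delay on Tick acts as a one-second clock that counts while the game mode's CombatStarted is set, triggering the win menu at five minutes.
; HUD creation is left unconnected.
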(event EventTick
  (params (DeltaSeconds :type Float%20%28single-precision%29))
  (bind _returnvalue (Game|GetPlayerController 0))
  (Utilities|FlowControl|Delay 1.0)
  (bind _asnew_game_mode_base (Utilities|Casting|CastToNewGameModeBase (Game|GetGameMode)))
  (if (Variables|/Script/COMP3000.NewGameModeBase|GetCombatStarted _asnew_game_mode_base)
    (Variables|Default|SetSeconds (+ (Variables|Default|GetSeconds) 1))
    (if (> (Variables|Default|GetSeconds) 59)
      (Variables|Default|SetMinutes (+ (Variables|Default|GetMinutes) 1))
      (Variables|Default|SetSeconds 0)
      (if (and (== (Variables|Default|GetMinutes) 5) (== (Variables|Default|GetSeconds) 0))
        (Game|SetGamePaused true)
        (bind _returnvalue_2 (UserInterface|CreateWidget "/Game/UI/WinMenu.WinMenu_C" _returnvalue))
        (UserInterface|Viewport|AddtoViewport _returnvalue_2 0)
        (Input|SetInputModeUIOnly _returnvalue 0 "DoNotLock" false)
        (Variables|/Script/Engine.PlayerController|SetbShowMouseCursor _returnvalue true)))))

(event EventDEATH
  (bind _returnvalue (Game|GetPlayerController 0))
  (bind _output_get (Variables|Default|SetIsGameOver true))
  (Game|SetGamePaused _output_get)
  (bind _returnvalue_2 (UserInterface|CreateWidget "/Game/UI/DeathMenu.DeathMenu_C" _returnvalue))
  (UserInterface|Viewport|AddtoViewport _returnvalue_2 0)
  (Input|SetInputModeUIOnly _returnvalue 0 "DoNotLock" false)
  (Variables|/Script/Engine.PlayerController|SetbShowMouseCursor _returnvalue true))

(event EventBeginPlay
  (bind _returnvalue (UserInterface|CreateWidget "/Game/UI/JumpMessage.JumpMessage_C"))
  (UserInterface|Viewport|AddtoViewport _returnvalue 0)
  (Input|SetInputModeGameOnly (Game|GetPlayerController 0) false))

(event EventLevelUpTRIGGER
  (bind _returnvalue (Game|GetPlayerController 0))
  (Variables|Default|SetIsGameOver false)
  (Game|SetGamePaused true)
  (bind _returnvalue_2 (UserInterface|CreateWidget "/Game/UI/LevelUP.LevelUP_C" _returnvalue))
  (UserInterface|Viewport|AddtoViewport _returnvalue_2 0)
  (Input|SetInputModeUIOnly _returnvalue 0 "DoNotLock" false)
  (Variables|/Script/Engine.PlayerController|SetbShowMouseCursor _returnvalue true))

(event Input|KeyboardEvents|Escape
  (params (Key :type Key%20Structure :default "None"))
  (bind _returnvalue (Game|GetPlayerController 0))
  (:Pressed
    (if (not (Variables|Default|GetIsGameOver))
      (bind _returnvalue_2 (UserInterface|CreateWidget "/Game/UI/PauseMenu.PauseMenu_C"))
      (Variables|Default|SetPause%20Menu%20Ref _returnvalue_2)
      (Variables|/Script/Engine.PlayerController|SetbShowMouseCursor _returnvalue true)
      (Input|SetInputModeUIOnly _returnvalue (Variables|Default|GetPause%20Menu%20Ref) "DoNotLock" false)
      (UserInterface|Viewport|AddtoViewport (Variables|Default|GetPause%20Menu%20Ref) 0)
      (Game|SetGamePaused true))))

(fn ConstructionScript)